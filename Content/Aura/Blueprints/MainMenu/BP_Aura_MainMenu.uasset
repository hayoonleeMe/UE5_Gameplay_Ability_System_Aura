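; BP_Aura_MainMenu is an actor, apparently for the main menu scene, that animates a floating fireball and a rotating magic circle decal.
; BeginPlay stores the fireball's start location, and each Tick offsets it vertically by a sine of accumulated time scaled by Amplitude.
; The time counter resets after passing two pi, while the decal rolls at a configurable rate scaled by world delta time.
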(event `self.ReceiveBeginPlay`
  (set `self.FireBallInitialLocation` (`SceneComponent.K2_GetComponentLocation` (`self.FireBall`))))

(event `self.ReceiveTick`
  (params (DeltaSeconds :type "Float (single-precision)"))
  (`self.UpdateTime` DeltaSeconds)
  (`SceneComponent.K2_SetWorldLocation` (`self.FireBall`) (+ (`self.FireBallInitialLocation`) (`KismetMathLibrary.MakeVector` 0.0 0.0 (`self.SinTime`))) false false)
  (`SceneComponent.K2_AddLocalRotation` (`self.MagicCircleDecal`) (`KismetMathLibrary.MakeRotator` (* (`GameplayStatics.GetWorldDeltaSeconds`) (`self.MagicCircleRoationRate`))) false false))

(fn `SinTime`
  (returns (ReturnValue :type "Float (double-precision)"))
  (return (* (`KismetMathLibrary.Sin` (`self.Time`)) (`self.Amplitude`))))

(fn `UpdateTime`
  (params (A :type "Float (double-precision)"))
  (bind _output_get (set `self.Time` (+ A (`self.Time`))))
  (if (> _output_get (`KismetMathLibrary.MultiplyByPi` 2.0))
    (set `self.Time` 0.0)))

(fn `UserConstructionScript`)